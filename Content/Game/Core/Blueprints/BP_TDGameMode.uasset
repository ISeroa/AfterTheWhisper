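; Game mode Blueprint that handles the end of a match, for both winning and losing.
; OnGameWon shows the WBP_ExtractionSuccess widget and OnGameLost shows WBP_GameOver.
; Both events then show the mouse cursor, switch the first player to UI-only input and pause the game.
; It holds no logic for deciding the outcome, and BeginPlay and the construction script are empty.
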(event `self.OnGameWon`
  (bind _returnvalue (`GameplayStatics.GetPlayerController` 0))
  (bind _returnvalue_2 (`|CreateWidget` "/Game/Game/UI/Result/WBP_ExtractionSuccess.WBP_ExtractionSuccess_C" (`GameplayStatics.GetPlayerController` 0)))
  (`UserWidget.AddToViewport` _returnvalue_2 0)
  (set `PlayerController.bShowMouseCursor` true _returnvalue)
  (`WidgetBlueprintLibrary.SetInputMode_UIOnlyEx` _returnvalue null)
  (`GameplayStatics.SetGamePaused` true))

(event `self.OnGameLost`
  (bind _returnvalue (`GameplayStatics.GetPlayerController` 0))
  (bind _returnvalue_2 (`|CreateWidget` "/Game/Game/UI/Result/WBP_GameOver.WBP_GameOver_C" (`GameplayStatics.GetPlayerController` 0)))
  (`UserWidget.AddToViewport` _returnvalue_2 0)
  (set `PlayerController.bShowMouseCursor` true _returnvalue)
  (`WidgetBlueprintLibrary.SetInputMode_UIOnlyEx` _returnvalue null)
  (`GameplayStatics.SetGamePaused` true))

(fn `UserConstructionScript`)